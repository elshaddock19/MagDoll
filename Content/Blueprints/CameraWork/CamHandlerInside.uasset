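; CamHandlerInside is a trigger actor that switches the player's view to a fixed camera while the MainCharacter is inside it.
; On begin overlap it blends the view target to each actor overlapping its DoorCam, calling OnEnter on the first CameraMaster found for each one.
; On end overlap it calls OnExit and returns the view to the controlled pawn once CameraMaster's collision count reaches zero or below.
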(event `self.ReceiveBeginPlay`)

(event `self.ReceiveActorBeginOverlap`
  (params (OtherActor :type "Actor Object Reference"))
  (if (`KismetMathLibrary.ClassIsChildOf` (`GameplayStatics.GetObjectClass` OtherActor) "/Game/Character/MainCharacter.MainCharacter_C")
    (`KismetSystemLibrary.PrintString` (`KismetSystemLibrary.GetObjectName` OtherActor))
    (for _array_element (`self.GetOverlappingActors` "/Game/Blueprints/CameraWork/DoorCam.DoorCam_C")
      (`KismetSystemLibrary.PrintString` (`KismetSystemLibrary.GetDisplayName` _array_element))
      (`PlayerController.SetViewTargetWithBlend` (`GameplayStatics.GetPlayerController` 0) _array_element 0.0 "VTBlend_Linear" 0.0 false)
      (bind _outactors (`GameplayStatics.GetAllActorsOfClass` "/Game/Blueprints/CameraWork/CameraMaster.CameraMaster_C"))
      (`/Game/Blueprints/CameraWork/CameraMaster.OnEnter` (`|GetArrayItem` _outactors)))))

(event `self.ReceiveActorEndOverlap`
  (params (OtherActor :type "Actor Object Reference"))
  (if (`KismetMathLibrary.ClassIsChildOf` (`GameplayStatics.GetObjectClass` OtherActor) "/Game/Character/MainCharacter.MainCharacter_C")
    (bind _outactors (`GameplayStatics.GetAllActorsOfClass` "/Game/Blueprints/CameraWork/CameraMaster.CameraMaster_C"))
    (bind _output (`|GetArrayItem` _outactors))
    (`/Game/Blueprints/CameraWork/CameraMaster.OnExit` _output)
    (bind _newparam (`/Game/Blueprints/CameraWork/CameraMaster.GetCamCollisions` _output))
    (`KismetSystemLibrary.PrintString` (`KismetStringLibrary.Conv_IntToString` _newparam))
    (if (<= _newparam 0)
      (`PlayerController.SetViewTargetWithBlend` (`GameplayStatics.GetPlayerController` 0) (`Controller.K2_GetPawn` (`GameplayStatics.GetPlayerController` 0)) 0.0 "VTBlend_Linear" 0.0 false))))

(fn `UserConstructionScript`)