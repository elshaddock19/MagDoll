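; Magnetic monopole actor that pushes or pulls its Pole component relative to components overlapping its ActionRange sphere.
; Each tick, ApplyInfluence applies force at the Pole's center of mass, falling quadratically from MaxForce to zero at the sphere's radius.
; The Pole's material, set at construction, acts as polarity: differing materials repel and matching ones attract.
; The force applied to each other component is zero, so only this Pole is moved.
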(event `self.ReceiveTick`
  (params (DeltaSeconds :type "Float (single-precision)"))
  (`self.ApplyInfluence` (`self.pole`) (`self.ActionRange`) (`SphereComponent.GetScaledSphereRadius` (`self.ActionRange`))))

(fn `ApplyInfluence`
  (params (pole :type "PrimitiveComponent Object Reference") (ActionRange :type "PrimitiveComponent Object Reference") (MaxDistance :type "Float (double-precision)"))
  (locals (L_Pole :type "PrimitiveComponent Object Reference") (L_ActionRange :type "PrimitiveComponent Object Reference") (L_ForeignPole :type "PrimitiveComponent Object Reference") (L_MaxDistance :type "Float (double-precision)"))
  (bind _l_maxdistance (`local.L_MaxDistance`))
  (bind _returnvalue (`PrimitiveComponent.GetCenterOfMass` (`local.L_ForeignPole`) "None"))
  (bind _returnvalue_2 (`PrimitiveComponent.GetCenterOfMass` (`local.L_Pole`) "None"))
  (bind _returnvalue_3 (- _returnvalue_2 _returnvalue))
  (set `local.L_Pole` pole)
  (set `local.L_ActionRange` ActionRange)
  (set `local.L_MaxDistance` MaxDistance)
  (for _array_element (`PrimitiveComponent.GetOverlappingComponents` (`local.L_ActionRange`))
    (bind _output_get (set `local.L_ForeignPole` _array_element))
    (if (!= _output_get (`local.L_Pole`))
      (`PrimitiveComponent.AddForceAtLocation` (`local.L_ForeignPole`) (0.0 0.0 0.0) _returnvalue "None")
      (`PrimitiveComponent.AddForceAtLocation` (`local.L_Pole`) (* (* (`KismetMathLibrary.Normal` _returnvalue_3) (* (`self.MaxForce`) (`KismetMathLibrary.Square` (/ (- _l_maxdistance (`KismetMathLibrary.FClamp` (`KismetMathLibrary.VSize` _returnvalue_3) 0.0 _l_maxdistance)) _l_maxdistance)))) (select `bool` (!= (`PrimitiveComponent.GetMaterial` (`local.L_ForeignPole`) 0) (`PrimitiveComponent.GetMaterial` (`local.L_Pole`) 0)) :`false` -1.0 :`true` 1.0 :!type "Float (single-precision)")) _returnvalue_2 "None"))))

(fn `UserConstructionScript`
  (`PrimitiveComponent.SetMaterial` (`self.pole`) 0 (`self.Material`)))